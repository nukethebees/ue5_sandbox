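; Small health pack actor Blueprint that gives its mesh a green glowing cross.
; The construction script runs the parent's script, then creates a dynamic instance of M_GlowingCross on the mesh's first material slot and sets its CrossColour parameter to green.
; The event graph holds only disabled default events, so the Blueprint adds no gameplay logic of its own there.
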(event EventBeginPlay
  (|CallParentFunction) ; This node is disabled and will not be called.\nDrag off pins to build functionality.
)

(event Collision|EventActorBeginOverlap
  (params (OtherActor :type Actor%20Object%20Reference))
  (|CallParentFunction OtherActor) ; This node is disabled and will not be called.\nDrag off pins to build functionality.
)

(event EventTick
  (params (DeltaSeconds :type Float%20%28single-precision%29))
  (|CallParentFunction DeltaSeconds) ; This node is disabled and will not be called.\nDrag off pins to build functionality.
)

(fn ConstructionScript
  (|CallParentFunction)
  (bind _returnvalue (Rendering|Material|CreateDynamicMaterialInstance (Variables|Default|Getmesh_component) 0 "/Game/Materials/M_GlowingCross.M_GlowingCross" "None" :!class /Script/Engine.PrimitiveComponent))
  (Rendering|Material|SetVectorParameterValue _returnvalue "CrossColour" (Class|KismetMathLibrary|LinearColorGreen) :!class /Script/Engine.MaterialInstanceDynamic))